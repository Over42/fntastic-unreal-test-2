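; Turtle actor that alternates between walking and pausing, with footstep audio following its state.
; Tick either calls Move scaled by Speed and delta time, or idles, based on the Wait flag.
; Latent Delays inside Tick flip Wait after MoveTime or WaitTime, so movement repeats each frame while the timer runs.
; Each flip sets the Footstep audio's IsWaiting parameter to match.
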(event EventBeginPlay
  (|CallParentFunction))

(event EventTick
  (params (DeltaSeconds :type Float%20%28single-precision%29))
  (|CallParentFunction DeltaSeconds)
  (if (Variables|Default|GetbWait)
    (Utilities|FlowControl|Delay (Variables|Default|GetWaitTime))
    (Variables|Default|SetbWait false)
    ;[1 1 1] AUDIO: Walking
    (Effects|Components|ParticleSystem|SetBoolParameter (Variables|Default|GetFootstep) "IsWaiting" false)
    (else
      (Class|Turtle|Move (* DeltaSeconds (Variables|Default|GetSpeed)))
      (Utilities|FlowControl|Delay (Variables|Default|GetMoveTime))
      (Variables|Default|SetbWait true)
      (Effects|Components|ParticleSystem|SetBoolParameter (Variables|Default|GetFootstep) "IsWaiting" true))))

(fn ConstructionScript
  (|CallParentFunction))