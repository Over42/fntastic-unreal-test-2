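; BP_Turtle_3 is a turtle Blueprint that moves back and forth, alternating between forward and backward phases.
; Each Tick calls Move with delta time scaled by Speed, negated while MoveBackward is set.
; Delay nodes on the Tick path flip MoveBackward after MoveForwardTime or MoveBackwardTime, while movement continues every frame.
; BeginPlay, Tick and the construction script all call their parent versions.
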(event EventBeginPlay
  (|CallParentFunction))

(event EventTick
  (params (DeltaSeconds :type Float%20%28single-precision%29))
  (|CallParentFunction DeltaSeconds)
  (if (Variables|Default|GetbMoveBackward)
    (Class|Turtle|Move (* DeltaSeconds (Variables|Default|GetSpeed) -1.0))
    (Utilities|FlowControl|Delay (Variables|Default|GetMoveBackwardTime))
    (Variables|Default|SetbMoveBackward false)
    (else
      (Class|Turtle|Move (* DeltaSeconds (Variables|Default|GetSpeed)))
      (Utilities|FlowControl|Delay (Variables|Default|GetMoveForwardTime))
      (Variables|Default|SetbMoveBackward true))))

(fn ConstructionScript
  (|CallParentFunction))